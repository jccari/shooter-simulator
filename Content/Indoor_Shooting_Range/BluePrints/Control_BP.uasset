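; Control actor for the indoor shooting range that drives a gate as the player approaches and leaves.
; A box trigger calls Open and Close on the gate when a FirstPersonCharacter begins or ends overlap.
; The G key calls Enter on the gate, while F only prints a debug string.
; BeginPlay stores the Cube's location in variables that nothing here reads.
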(event OnComponentBeginOverlap(Box)
  (params (OverlappedComponent :type Primitive%20Component%20Object%20Reference) (OtherActor :type Actor%20Object%20Reference) (OtherComp :type Primitive%20Component%20Object%20Reference) (OtherBodyIndex :type Integer) (bFromSweep :type Boolean) (SweepResult :type Hit%20Result%20Structure%20%28by%20ref%29))
  (Utilities|Casting|CastToFirstPersonCharacter OtherActor)
  (Utilities|FlowControl|Gate true) ; enters at Open
)

(event OnComponentEndOverlap(Box)
  (params (OverlappedComponent :type Primitive%20Component%20Object%20Reference) (OtherActor :type Actor%20Object%20Reference) (OtherComp :type Primitive%20Component%20Object%20Reference) (OtherBodyIndex :type Integer))
  (Utilities|Casting|CastToFirstPersonCharacter OtherActor)
  (Utilities|FlowControl|Gate true) ; enters at Close
)

(event Custom|CustomEvent_0
  (Variables|Default|Setnew%20location (Transformation|GetActorLocation (Variables|Default|Getcube%20?))))

(event EventBeginPlay
  (bind _cube__ (Variables|Default|Getcube%20?))
  (bind _returnvalue (Transformation|GetActorLocation _cube__))
  (Variables|Default|SetNewVar_0 (.X (Math|Vector|BreakVector _returnvalue)))
  (Variables|Default|Setdefault%20location _returnvalue)
  (Variables|Default|Setnew%20location (Transformation|GetActorLocation (Variables|Default|Getcube%20?))))

(event Input|KeyboardEvents|F
  (params (Key :type Key%20Structure :default "None"))
  (:Pressed
    (Development|PrintString "touch F")))

(event Input|KeyboardEvents|G
  (params (Key :type Key%20Structure :default "None"))
  (:Pressed
    (Utilities|FlowControl|Gate true)))

(fn ConstructionScript)